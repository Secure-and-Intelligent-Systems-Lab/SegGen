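; Character Blueprint with input actions for dataset capture: toggling a depth-modality cube, applying label materials and playing the CollectDataset1 level sequence.
; The labels action walks actors of each Sections class, passing substring-to-material pairs from Classes (Trees, Plants, Rocks, Other) to PaintItems.
; The Other pass leaves PaintItems' Section input unset.
; PaintItems and ReturnToOriginal, called by the reset action, have empty bodies here.
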(event Input|EnhancedActionEvents|EnhancedInputActionIA_Labels
  (params (ActionValue :type Boolean) (ElapsedSeconds :type Float%20%28double-precision%29) (TriggeredSeconds :type Float%20%28double-precision%29) (InputAction :type Input%20Action%20Object%20Reference :default "/Game/Input/IA_Labels.IA_Labels"))
  (bind _classes (Variables|Default|GetClasses))
  (bind _classes_2 (Variables|Default|GetClasses))
  (bind _classes_3 (Variables|Default|GetClasses))
  (bind _classes_4 (Variables|Default|GetClasses))
  (bind _other (Utilities|Struct|BreakClasses _classes_2))
  (bind _trees (Utilities|Struct|BreakClasses _classes_3))
  (bind _plants (Utilities|Struct|BreakClasses _classes_4))
  (bind _rocks (Utilities|Struct|BreakClasses _classes))
  (:Started
    (Utilities|FlowControl|Sequence
      (:then_0
        (for _array_element (Variables|Default|GetSections)
          (bind _outactors (Actor|GetAllActorsOfClass _array_element))
          (for _array_element_2 _outactors
            (bind _keys (Utilities|Map|Keys _trees))
            (for _array_element_3 _keys
              (CallFunction|PaintItems _array_element_3 _array_element_2 (.Value (Utilities|Map|Find _trees _array_element_3)))))))
      (:then_1
        (for _array_element_4 (Variables|Default|GetSections)
          (bind _outactors_2 (Actor|GetAllActorsOfClass _array_element_4))
          (for _array_element_5 _outactors_2
            (bind _keys_2 (Utilities|Map|Keys _plants))
            (for _array_element_6 _keys_2
              (CallFunction|PaintItems _array_element_6 _array_element_5 (.Value (Utilities|Map|Find _plants _array_element_6)))))))
      (:then_2
        (for _array_element_7 (Variables|Default|GetSections)
          (bind _outactors_3 (Actor|GetAllActorsOfClass _array_element_7))
          (for _array_element_8 _outactors_3
            (bind _keys_3 (Utilities|Map|Keys _rocks))
            (for _array_element_9 _keys_3
              (CallFunction|PaintItems _array_element_9 _array_element_8 (.Value (Utilities|Map|Find _rocks _array_element_9)))))))
      (:then_3
        (for _array_element_10 (Variables|Default|GetSections)
          (bind _outactors_4 (Actor|GetAllActorsOfClass _array_element_10))
          (for _array_element_11 _outactors_4
            (bind _keys_4 (Utilities|Map|Keys _other))
            (for _array_element_12 _keys_4
              (CallFunction|PaintItems _array_element_12 0 (.Value (Utilities|Map|Find _other _array_element_12))))))))))

(event Input|EnhancedActionEvents|EnhancedInputActionIA_ReturnToOriginal
  (params (ActionValue :type Boolean) (ElapsedSeconds :type Float%20%28double-precision%29) (TriggeredSeconds :type Float%20%28double-precision%29) (InputAction :type Input%20Action%20Object%20Reference :default "/Game/Input/IA_ReturnToOriginal.IA_ReturnToOriginal"))
  (:Started
    (CallFunction|ReturntoOriginal)))

(event Input|EnhancedActionEvents|EnhancedInputActionIA_PlayDataset1
  (params (ActionValue :type Boolean) (ElapsedSeconds :type Float%20%28double-precision%29) (TriggeredSeconds :type Float%20%28double-precision%29) (InputAction :type Input%20Action%20Object%20Reference :default "/Game/Input/IA_PlayDataset1.IA_PlayDataset1"))
  (:Started
    (bind _returnvalue (Sequencer|Player|CreateLevelSequencePlayer "/Game/Blueprints/Sequences/CollectDataset1.CollectDataset1"))
    (Sequencer|Player|Play _returnvalue :!class /Script/MovieScene.MovieSceneSequencePlayer)))

(event Input|EnhancedActionEvents|EnhancedInputActionIA_DepthModality
  (params (ActionValue :type Boolean) (ElapsedSeconds :type Float%20%28double-precision%29) (TriggeredSeconds :type Float%20%28double-precision%29) (InputAction :type Input%20Action%20Object%20Reference :default "/Game/Input/IA_DepthModality.IA_DepthModality"))
  (:Started
    (Rendering|ToggleVisibility (Variables|Default|GetDepthModalityCube) false)))

(event EventBeginPlay)

(event Collision|EventActorBeginOverlap
  (params (OtherActor :type Actor%20Object%20Reference)))

(event EventTick
  (params (DeltaSeconds :type Float%20%28single-precision%29)))

(fn ConstructionScript)

(fn PaintItems
  (params (Substring :type String) (Section :type Actor%20Object%20Reference) (Material :type Material%20Instance%20Object%20Reference)))

(fn ReturntoOriginal)